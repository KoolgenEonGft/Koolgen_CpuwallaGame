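; Game mode for a keyboard level, holding six rows of key lights and helper logic to step through them.
; Motionmaker advances a row/column cursor in a serpentine path, reversing direction on each row and looking up each light through Givethepointlight, whose result it leaves unused.
; UMFGiveTheRow maps a row number to its array.
; BeginPlay is empty, and the color, intensity, timeline and Motionmaker test calls in the event graph never run.
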(event `self.ReceiveBeginPlay`)

(fn `Givethepointlight`
  (params (RowNUm :type Integer) (ColumnNUm :type Integer))
  (returns (pointlightcomp :type "PointLightComponent Object Reference"))
  (switch `int` RowNUm
    (:`0`
      (return (`|GetArrayItem` (`self.Row0`) ColumnNUm)))
    (:`1`
      (return (`|GetArrayItem` (`self.Row1`) ColumnNUm)))
    (:`2`
      (return (`|GetArrayItem` (`self.Row2`) ColumnNUm)))
    (:`3`
      (return (`|GetArrayItem` (`self.Row3`) ColumnNUm)))
    (:`4`
      (return (`|GetArrayItem` (`self.Row4`) ColumnNUm)))
    (:`5`
      (return (`|GetArrayItem` (`self.Row5`) ColumnNUm)))))

(fn `Motionmaker`
  (if (`self.StraightOrNot`)
    (bind _pointlightrow (`self.UMF_GiveTheRow` (`self.TopRowNO`)))
    (if (< (`self.TopColumnNo`) (- (`KismetArrayLibrary.Array_Length` _pointlightrow) 1))
      (`/Engine/EditorBlueprintResources/StandardMacros.IncrementInt` (`self.TopColumnNo`)
        (:`  `
          (`self.Givethepointlight` (`self.TopRowNO`) (`self.TopColumnNo`))))
      (else
        (`/Engine/EditorBlueprintResources/StandardMacros.IncrementInt` (`self.TopRowNO`)
          (:`  `
            (if (< (`self.TopRowNO`) 6)
              (bind _pointlightrow_2 (`self.UMF_GiveTheRow` (`self.TopRowNO`)))
              (set `self.TopColumnNo` (- (`KismetArrayLibrary.Array_Length` _pointlightrow_2) 1))
              (set `self.StraightOrNot` false)
              (`self.Givethepointlight` (`self.TopRowNO`) (`self.TopColumnNo`)))))))
    (elif (> (`self.TopColumnNo`) 0)
      (`/Engine/EditorBlueprintResources/StandardMacros.DecrementInt` (`self.TopColumnNo`)
        (:`  `
          (`self.Givethepointlight` (`self.TopRowNO`) (`self.TopColumnNo`))))
      (else
        (bind _result (`/Engine/EditorBlueprintResources/StandardMacros.IncrementInt` (`self.TopRowNO`))
          (:`  `
            (if (< _result 6)
              (`self.UMF_GiveTheRow` (`self.TopRowNO`))
              (set `self.TopColumnNo` 0)
              (set `self.StraightOrNot` true)
              (`self.Givethepointlight` (`self.TopRowNO`) (`self.TopColumnNo`)))))))))

(fn `UMF_GiveTheRow`
  (params (RowNumber :type Integer :default 0))
  (returns (PointLightRow :type "Array of PointLightComponent Object Reference"))
  (switch `int` RowNumber
    (:`0`
      (return (`self.Row0`)))
    (:`1`
      (return (`self.Row1`)))
    (:`2`
      (return (`self.Row2`)))
    (:`3`
      (return (`self.Row3`)))
    (:`4`
      (return (`self.Row4`)))
    (:`5`
      (return (`self.Row5`)))))

(fn `UserConstructionScript`)