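; Snake movement component that lays out and advances a snake of lit cells on a row-and-column grid owned by the game mode.
; BeginPlay seeds a length-clamped body from the top or bottom start cell, lights it through game mode interface messages, then inserts one head cell.
; Separate functions add head cells and remove tail cells, with no Tick logic driving them.
; At row ends the head changes row, wrapping after the last, and flips direction.
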(event `self.ReceiveBeginPlay`
  (bind _returnvalue (- (`self.IVAR_INT_SnakesBodyLength`) 1))
  (bind _returnvalue_2 (- 7 (`self.IVAR_INT_SnakesBodyLength`)))
  (set `self.GVAR_GMO_GameModeSoftRefrence` (`GameplayStatics.GetGameMode`))
  (set `self.IVAR_BOOL_GoingFoward` (`self.IVAR_BOOL_StartFromTop?`))
  (if (`self.IVAR_BOOL_StartFromTop?`)
    (set `self.IVAR_INT_SnakesBodyLength` (`KismetMathLibrary.Clamp` (`self.IVAR_INT_SnakesBodyLength`) 1 13))
    (set `self.IVAR_STR_SnakesBodyBottomPart` (make `/Game/GameContent/Structures/UMSTR_SnakesBodyPart/UMSTR_SnakesBodyPart_BP` 0))
    (for _index (range (+ _returnvalue 1))
      (message `/Game/GameContent/BlueprintInterface/UMBINF_SnakeMovementComponent_GameMode/UMBINF_SnakeMovementComponent_GameMode_ACTPointlightBP.INFUN_SetTheLIghtsON` (`self.GVAR_GMO_GameModeSoftRefrence`) 0 _index)
      (`KismetArrayLibrary.Array_Add` (`self.IVAR_STR_SnakesBody`) (make `/Game/GameContent/Structures/UMSTR_SnakesBodyPart/UMSTR_SnakesBodyPart_BP` 0 _index)))
    (set `self.IVAR_STR_SnakesBodyTopPart` (make `/Game/GameContent/Structures/UMSTR_SnakesBodyPart/UMSTR_SnakesBodyPart_BP` 0 _returnvalue))
    (`self.UMF_InsertTheTopBodyPart`)
    (else
      (set `self.IVAR_INT_SnakesBodyLength` (`KismetMathLibrary.Clamp` (`self.IVAR_INT_SnakesBodyLength`) 1 7))
      (set `self.IVAR_STR_SnakesBodyBottomPart` (make `/Game/GameContent/Structures/UMSTR_SnakesBodyPart/UMSTR_SnakesBodyPart_BP` 5 7))
      (for _index_2 (range -7 (+ (* _returnvalue_2 -1) 1))
        (bind _returnvalue_3 (`KismetMathLibrary.Abs_Int` _index_2))
        (message `/Game/GameContent/BlueprintInterface/UMBINF_SnakeMovementComponent_GameMode/UMBINF_SnakeMovementComponent_GameMode_ACTPointlightBP.INFUN_SetTheLIghtsON` (`self.GVAR_GMO_GameModeSoftRefrence`) 5 _returnvalue_3)
        (`KismetArrayLibrary.Array_Add` (`self.IVAR_STR_SnakesBody`) (make `/Game/GameContent/Structures/UMSTR_SnakesBodyPart/UMSTR_SnakesBodyPart_BP` 5 _returnvalue_3)))
      (set `self.IVAR_STR_SnakesBodyTopPart` (make `/Game/GameContent/Structures/UMSTR_SnakesBodyPart/UMSTR_SnakesBodyPart_BP` 5 _returnvalue_2))
      (`self.UMF_InsertTheTopBodyPart`))))

(fn `INFUN_GetTheLengthOfTheRow`
  (params (LVAR_INT_RowNumber :type Integer))
  (returns (LVAR_INT_LengthOfTheRow :type Integer))
  (return 0))

(fn `UMF_ChnageTheRowAccordingToTheCategory`
  (params (LVAR_INT_RowNumber :type Integer))
  (returns (IVAR_INT_NewRowNumber :type Integer) (IVAR_INT_NewColumnNumber :type Integer))
  (bind _returnvalue (- (`local.LVAR_INT_RowNumber`) 1))
  (bind _returnvalue_2 (+ (`local.LVAR_INT_RowNumber`) 1))
  (if (`self.IVAR_BOOL_StartFromTop?`)
    (if (< _returnvalue_2 6)
      (bind _lvar_int_lengthoftherow (message `/Game/GameContent/BlueprintInterface/UMBINF_SnakeMovementComponent_GameMode/UMBINF_SnakeMovementComponent_GameMode_ACTPointlightBP.INFUN_GetTheLengthOfTheRow` (`self.GVAR_GMO_GameModeSoftRefrence`) _returnvalue_2))
      (return _returnvalue_2 (- _lvar_int_lengthoftherow 1))
      (else
        (return 0 0)))
    (elif (>= _returnvalue 0)
      (return _returnvalue 0)
      (else
        (return 5 7)))))

(fn `UMF_DeleteTheBottomBodyPart`
  (bind _ivar_str_snakesbody (`self.IVAR_STR_SnakesBody`))
  (bind (_rownumber _columnnumber) (break `/Game/GameContent/Structures/UMSTR_SnakesBodyPart/UMSTR_SnakesBodyPart_BP` (`self.IVAR_STR_SnakesBodyBottomPart`)))
  (message `/Game/GameContent/BlueprintInterface/UMBINF_SnakeMovementComponent_GameMode/UMBINF_SnakeMovementComponent_GameMode_ACTPointlightBP.INFUN_ToggleVisibiltyOff` (`self.GVAR_GMO_GameModeSoftRefrence`) _rownumber _columnnumber (`self.IVAR_INT_SnakeIndexNo`))
  (`KismetArrayLibrary.Array_Remove` _ivar_str_snakesbody)
  (set `self.IVAR_STR_SnakesBodyBottomPart` (`|GetArrayItem` _ivar_str_snakesbody)))

(fn `UMF_InsertTheTopBodyPart`
  (bind (_rownumber _columnnumber) (break `/Game/GameContent/Structures/UMSTR_SnakesBodyPart/UMSTR_SnakesBodyPart_BP` (`self.IVAR_STR_SnakesBodyTopPart`)))
  (bind (_rownumber_2 _columnnumber_2) (break `/Game/GameContent/Structures/UMSTR_SnakesBodyPart/UMSTR_SnakesBodyPart_BP` (`self.IVAR_STR_SnakesBodyTopPart`)))
  (bind (_rownumber_3 _columnnumber_3) (break `/Game/GameContent/Structures/UMSTR_SnakesBodyPart/UMSTR_SnakesBodyPart_BP` (`self.IVAR_STR_SnakesBodyTopPart`)))
  (bind _returnvalue (- _columnnumber_3 1))
  (bind _returnvalue_2 (+ _columnnumber_2 1))
  (bind _umstr_snakesbodypart_bp (make `/Game/GameContent/Structures/UMSTR_SnakesBodyPart/UMSTR_SnakesBodyPart_BP` _rownumber_3 _returnvalue))
  (bind _umstr_snakesbodypart_bp_2 (make `/Game/GameContent/Structures/UMSTR_SnakesBodyPart/UMSTR_SnakesBodyPart_BP` _rownumber_2 _returnvalue_2))
  (if (`self.IVAR_BOOL_GoingFoward`)
    (bind _lvar_int_lengthoftherow (message `/Game/GameContent/BlueprintInterface/UMBINF_SnakeMovementComponent_GameMode/UMBINF_SnakeMovementComponent_GameMode_ACTPointlightBP.INFUN_GetTheLengthOfTheRow` (`self.GVAR_GMO_GameModeSoftRefrence`) _rownumber))
    (if (< (+ _columnnumber 1) _lvar_int_lengthoftherow)
      (message `/Game/GameContent/BlueprintInterface/UMBINF_SnakeMovementComponent_GameMode/UMBINF_SnakeMovementComponent_GameMode_ACTPointlightBP.INFUN_ToggleVisibiltyOn` (`self.GVAR_GMO_GameModeSoftRefrence`) _rownumber_2 _returnvalue_2 (`self.IVAR_INT_SnakeIndexNo`))
      (`KismetArrayLibrary.Array_Add` (`self.IVAR_STR_SnakesBody`) _umstr_snakesbodypart_bp_2)
      (set `self.IVAR_STR_SnakesBodyTopPart` _umstr_snakesbodypart_bp_2)
      (else
        (bind (_ivar_int_newrownumber _ivar_int_newcolumnnumber) (`self.UMF_ChnageTheRowAccordingToTheCategory` _rownumber))
        (message `/Game/GameContent/BlueprintInterface/UMBINF_SnakeMovementComponent_GameMode/UMBINF_SnakeMovementComponent_GameMode_ACTPointlightBP.INFUN_ToggleVisibiltyOn` (`self.GVAR_GMO_GameModeSoftRefrence`) _ivar_int_newrownumber _ivar_int_newcolumnnumber (`self.IVAR_INT_SnakeIndexNo`))
        (bind _umstr_snakesbodypart_bp_3 (make `/Game/GameContent/Structures/UMSTR_SnakesBodyPart/UMSTR_SnakesBodyPart_BP` _ivar_int_newrownumber _ivar_int_newcolumnnumber))
        (`KismetArrayLibrary.Array_Add` (`self.IVAR_STR_SnakesBody`) _umstr_snakesbodypart_bp_3)
        (set `self.IVAR_STR_SnakesBodyTopPart` _umstr_snakesbodypart_bp_3)
        (set `self.IVAR_BOOL_GoingFoward` (not (`self.IVAR_BOOL_GoingFoward`)))))
    (elif (>= (- (`.ColumnNumber_6_3C265AF8488C7A92540C4CB2FE63A8BF` (break `/Game/GameContent/Structures/UMSTR_SnakesBodyPart/UMSTR_SnakesBodyPart_BP` (`self.IVAR_STR_SnakesBodyTopPart`))) 1) 0)
      (message `/Game/GameContent/BlueprintInterface/UMBINF_SnakeMovementComponent_GameMode/UMBINF_SnakeMovementComponent_GameMode_ACTPointlightBP.INFUN_ToggleVisibiltyOn` (`self.GVAR_GMO_GameModeSoftRefrence`) _rownumber_3 _returnvalue (`self.IVAR_INT_SnakeIndexNo`))
      (`KismetArrayLibrary.Array_Add` (`self.IVAR_STR_SnakesBody`) _umstr_snakesbodypart_bp)
      (set `self.IVAR_STR_SnakesBodyTopPart` _umstr_snakesbodypart_bp)
      (else
        (bind (_ivar_int_newrownumber_2 _ivar_int_newcolumnnumber_2) (`self.UMF_ChnageTheRowAccordingToTheCategory` (`.RowNumber_5_8B6731594E65AF3829383A8C5EA3B364` (break `/Game/GameContent/Structures/UMSTR_SnakesBodyPart/UMSTR_SnakesBodyPart_BP` (`self.IVAR_STR_SnakesBodyTopPart`)))))
        (message `/Game/GameContent/BlueprintInterface/UMBINF_SnakeMovementComponent_GameMode/UMBINF_SnakeMovementComponent_GameMode_ACTPointlightBP.INFUN_ToggleVisibiltyOn` (`self.GVAR_GMO_GameModeSoftRefrence`) _ivar_int_newrownumber_2 _ivar_int_newcolumnnumber_2 (`self.IVAR_INT_SnakeIndexNo`))
        (bind _umstr_snakesbodypart_bp_4 (make `/Game/GameContent/Structures/UMSTR_SnakesBodyPart/UMSTR_SnakesBodyPart_BP` _ivar_int_newrownumber_2 _ivar_int_newcolumnnumber_2))
        (`KismetArrayLibrary.Array_Add` (`self.IVAR_STR_SnakesBody`) _umstr_snakesbodypart_bp_4)
        (set `self.IVAR_STR_SnakesBodyTopPart` _umstr_snakesbodypart_bp_4)
        (set `self.IVAR_BOOL_GoingFoward` (not (`self.IVAR_BOOL_GoingFoward`)))))))