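; Breathing effect component that drives a color-cycling, pulsing effect on all buttons through the game mode.
; BeginPlay caches the game mode and initial play rate, and clamps the rate-increase factor.
; Each cycle call sends the current spectrum color and play rate to the game mode via interface messages, then advances the wrapping color index.
; The play rate only resets on an exact doubling check; nothing here increases it.
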(event `self.ReceiveBeginPlay`
  (set `self.GVAR_FL_IntialPlayRate` (`self.GVAR_FL_PlayRate`))
  (set `self.GVAR_FL_PlayRateIncreasingRate` (`KismetMathLibrary.FClamp` (`self.GVAR_FL_PlayRateIncreasingRate`) 0.01 0.1))
  (set `self.GVAR_GMO_GameModeRefrence` (`GameplayStatics.GetGameMode`)))

(fn `UMF_HandleTheColorChangeCycle`
  (message `/Game/GameContent/BlueprintInterface/UMBINF_SnakeMovementComponent_GameMode/UMBINF_SnakeMovementComponent_GameMode_ACTPointlightBP.INFUN_ChangeColorForAllButtons(BreathingEffectComponentToGameMode)` (`self.GVAR_GMO_GameModeRefrence`) (`|GetArrayItem` (`self.GAAR_LNC_ColorSpectrum`) (`self.GVAR_INT_CurrentColorIndex`)))
  (message `/Game/GameContent/BlueprintInterface/UMBINF_SnakeMovementComponent_GameMode/UMBINF_SnakeMovementComponent_GameMode_ACTPointlightBP.INFUN_ToggleVisibiltyOnForAllButtons(BreathingEffectComponentToGameMode)` (`self.GVAR_GMO_GameModeRefrence`) (`self.GVAR_FL_PlayRate`))
  (if (== (+ (`self.GVAR_FL_PlayRate`) (* (`self.GVAR_FL_PlayRate`) (`self.GVAR_FL_PlayRateIncreasingRate`))) (* (`self.GVAR_FL_IntialPlayRate`) 2.0))
    (set `self.GVAR_FL_PlayRate` (`self.GVAR_FL_IntialPlayRate`)))
  (bind _result (`/Engine/EditorBlueprintResources/StandardMacros.IncrementInt` (`self.GVAR_INT_CurrentColorIndex`))
    (:`  `
      (if (== _result (`KismetArrayLibrary.Array_Length` (`self.GAAR_LNC_ColorSpectrum`)))
        (set `self.GVAR_INT_CurrentColorIndex` 0)))))