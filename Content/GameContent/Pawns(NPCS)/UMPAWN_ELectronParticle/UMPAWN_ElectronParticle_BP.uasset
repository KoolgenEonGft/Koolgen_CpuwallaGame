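; Electron particle pawn that renders a tinted sphere with four spline-mesh effects offset around it.
; The construction script colors the sphere through a dynamic material using color and illumination variables, then adds the spline meshes.
; A shared helper gives each spline its own dynamic material, varying only speed between them.
; On BeginPlay, a timeline animates the end position of the first spline only.
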(event `self.ReceiveBeginPlay`
  (bind (_direction _x_axis _y_acis _newtrack_3) (`Timeline|Timeline_0`)
    (:`Update`
      (`SplineMeshComponent.SetEndPosition` (`self.NewVar_0`) (`KismetMathLibrary.MakeVector` _x_axis _y_acis _newtrack_3) true))))

(fn `UMF_GeneratingDynamicFunctions`
  (params (selfRefrence :type "SplineMeshComponent Object Reference") (Scale :type "Float (double-precision)") (Speed :type "Float (double-precision)") (MaskMult :type "Float (double-precision)") (MaskPower :type "Float (double-precision)") (DepthThickness :type "Float (double-precision)") (Displace :type "Float (double-precision)") (Opacity :type "Float (double-precision)") (Color :type "LinearColor Structure"))
  (bind _returnvalue (`PrimitiveComponent.CreateDynamicMaterialInstance` selfRefrence 0 null "None"))
  (`MaterialInstanceDynamic.SetScalarParameterValue` _returnvalue "Scale" Scale)
  (`MaterialInstanceDynamic.SetScalarParameterValue` _returnvalue "Speed" Speed)
  (`MaterialInstanceDynamic.SetScalarParameterValue` _returnvalue "Mask Mult" MaskMult)
  (`MaterialInstanceDynamic.SetScalarParameterValue` _returnvalue "Mask Power" MaskPower)
  (`MaterialInstanceDynamic.SetScalarParameterValue` _returnvalue "Depth Thicken" DepthThickness)
  (`MaterialInstanceDynamic.SetScalarParameterValue` _returnvalue "Displace" Displace)
  (`MaterialInstanceDynamic.SetScalarParameterValue` _returnvalue "Opacity" Opacity)
  (`MaterialInstanceDynamic.SetVectorParameterValue` _returnvalue "Color" Color))

(fn `UserConstructionScript`
  (bind (_r _g _b) (break `LinearColor` (`self.GVAR_LNC_LinearColor`)))
  (bind _returnvalue (`PrimitiveComponent.CreateDynamicMaterialInstance` (`self.Sphere`) 0 null "None"))
  (`MaterialInstanceDynamic.SetVectorParameterValue` _returnvalue "Color" (make `LinearColor` _r _g _b (`self.GVAR_FL_Illumination`)))
  (bind _returnvalue_2 (`AddComponent|NODE_AddSplineMeshComponent-0` :`RelativeTransform` (`KismetMathLibrary.MakeTransform` (0.0 27.0 30.0))))
  (bind _output_get (set `self.NewVar_0` _returnvalue_2))
  (`SplineMeshComponent.SetEndPosition` _output_get (`self.End Pos`) true)
  (`self.UMF_GeneratingDynamicFunctions` _returnvalue_2 46.0 5.0 1.0 1.52 0.0 9.3 1.0 (struct :`R` 1.0 :`G` 1.0 :`B` 1.0 :`A` 1.0))
  (bind _returnvalue_3 (`AddComponent|NODE_AddSplineMeshComponent-1` :`RelativeTransform` (`KismetMathLibrary.MakeTransform` (0.0 -27.0 38.0))))
  (`self.UMF_GeneratingDynamicFunctions` _returnvalue_3 46.0 7.0 1.0 1.52 0.0 9.3 1.0 (struct :`R` 1.0 :`G` 1.0 :`B` 1.0 :`A` 1.0))
  (bind _returnvalue_4 (`AddComponent|NODE_AddSplineMeshComponent-2` :`RelativeTransform` (`KismetMathLibrary.MakeTransform` (0.0 -27.0 -33.0))))
  (`self.UMF_GeneratingDynamicFunctions` _returnvalue_4 46.0 9.0 1.0 1.52 0.0 9.3 1.0 (struct :`R` 1.0 :`G` 1.0 :`B` 1.0 :`A` 1.0))
  (bind _returnvalue_5 (`AddComponent|NODE_AddSplineMeshComponent-3` :`RelativeTransform` (`KismetMathLibrary.MakeTransform` (0.0 27.0 -36.0))))
  (`self.UMF_GeneratingDynamicFunctions` _returnvalue_5 46.0 11.0 1.0 1.52 0.0 9.3 1.0 (struct :`R` 1.0 :`G` 1.0 :`B` 1.0 :`A` 1.0)))