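; Electron particle pawn built from a glowing sphere and an electric arc, configured entirely in the construction script.
; The script tints the sphere's dynamic material, using illumination as alpha, and adds a spline mesh stretched to EndPos.
; UMFGeneratingDynamicFunctions gives the arc a dynamic material driven by variables for shape, motion, opacity and color.
; Runtime events are empty; timeline animation and extra-arc experiments are disconnected.
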(event `self.ReceiveBeginPlay`)

(fn `UMF_GeneratingDynamicFunctions`
  (params (selfRefrence :type "SplineMeshComponent Object Reference") (Scale :type "Float (double-precision)") (Speed :type "Float (double-precision)") (MaskMult :type "Float (double-precision)") (MaskPower :type "Float (double-precision)") (DepthThickness :type "Float (double-precision)") (Displace :type "Float (double-precision)") (Opacity :type "Float (double-precision)") (Color :type "LinearColor Structure"))
  (bind _returnvalue (`PrimitiveComponent.CreateDynamicMaterialInstance` selfRefrence 0 null "None"))
  (`MaterialInstanceDynamic.SetScalarParameterValue` _returnvalue "Scale" Scale)
  (`MaterialInstanceDynamic.SetScalarParameterValue` _returnvalue "Speed" Speed)
  (`MaterialInstanceDynamic.SetScalarParameterValue` _returnvalue "Mask Mult" MaskMult)
  (`MaterialInstanceDynamic.SetScalarParameterValue` _returnvalue "Mask Power" MaskPower)
  (`MaterialInstanceDynamic.SetScalarParameterValue` _returnvalue "Depth Thicken" DepthThickness)
  (`MaterialInstanceDynamic.SetScalarParameterValue` _returnvalue "Displace" Displace)
  (`MaterialInstanceDynamic.SetScalarParameterValue` _returnvalue "Opacity" Opacity)
  (`MaterialInstanceDynamic.SetVectorParameterValue` _returnvalue "Color" Color))

(fn `UserConstructionScript`
  (bind (_r _g _b) (break `LinearColor` (`self.GVAR_LNC_LinearColor`)))
  (bind _returnvalue (`PrimitiveComponent.CreateDynamicMaterialInstance` (`self.Sphere`) 0 null "None"))
  (`MaterialInstanceDynamic.SetVectorParameterValue` _returnvalue "Color" (make `LinearColor` _r _g _b (`self.GVAR_FL_Illumination`)))
  (bind _returnvalue_2 (`AddComponent|NODE_AddSplineMeshComponent-6`))
  (`SplineMeshComponent.SetEndPosition` _returnvalue_2 (`self.End Pos`) true)
  (`self.UMF_GeneratingDynamicFunctions` _returnvalue_2 (`self.GVAR_FL_ArcScale`) (`self.GVAR_FL_ArcSpeed`) (`self.GVAR_FL_MaskMult`) (`self.GVAR_FL_Mask Power`) (`self.GVAR_FL_DepthThickeness`) (`self.GVAR_FL_Displace`) (`self.GVAR_FL_Opacity`) (`self.GVAR_LNC_Color`)))