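; ACT_Key_BP is a key actor whose cap mesh can be moved down and back up, like a key press and release.
; Custom fall and rise events each record the cap's current world location and offset its Z by a fall-height variable to get the target.
; Each then plays its own timeline, lerping the cap between those two positions along the timeline curve.
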(event `EVE_MakeKeyCapFall`
  (bind _returnvalue (`SceneComponent.K2_GetComponentLocation` (`self.STMC_KeyCap`)))
  (set `self.Var_VC_KeyCapIntialLoc` _returnvalue)
  (set `self.Var_VC_KeyCapFInalLoc` (`KismetMathLibrary.MakeVector` (.x _returnvalue) (.y _returnvalue) (- (.z _returnvalue) (`self.Var_Fl_FallHieght`))))
  (bind (_direction _keycapfallgraph) (`Timeline|Make KeyCapFallTimeline` :!via `PlayFromStart`)
    (:`Update`
      (`SceneComponent.K2_SetWorldLocation` (`self.STMC_KeyCap`) (`KismetMathLibrary.VLerp` (`self.Var_VC_KeyCapIntialLoc`) (`self.Var_VC_KeyCapFInalLoc`) _keycapfallgraph) false false))))

(event `Eve_MakeKeyCapRise`
  (bind _returnvalue (`SceneComponent.K2_GetComponentLocation` (`self.STMC_KeyCap`)))
  (set `self.Var_VC_KeyCapIntialLoc` _returnvalue)
  (set `self.Var_VC_KeyCapFInalLoc` (`KismetMathLibrary.MakeVector` (.x _returnvalue) (.y _returnvalue) (+ (.z _returnvalue) (`self.Var_Fl_FallHieght`))))
  (bind (_direction _keycapfallgraph) (`Timeline|MakeKeyCapRiseTImeline` :!via `PlayFromStart`)
    (:`Update`
      (`SceneComponent.K2_SetWorldLocation` (`self.STMC_KeyCap`) (`KismetMathLibrary.VLerp` (`self.Var_VC_KeyCapIntialLoc`) (`self.Var_VC_KeyCapFInalLoc`) _keycapfallgraph) false false))))

(fn `UserConstructionScript`)