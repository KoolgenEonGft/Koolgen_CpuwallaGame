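; Point light actor that exposes events to set its color and fade its intensity for default, snake and breathing lighting modes.
; Each fade plays a timeline at a given play rate, scaling its curve by a global intensity.
; Snake events range-check intensity, then either fade or wait one over the play rate.
; They then notify the game mode with the snake index, so it knows the step is done.
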(event `UMEVE_ChangeColor`
  (params (LVAR_LNC_ChangingColor :type "LinearColor Structure"))
  ;[0 0 0 1 15] Changing the Color Of The Each Point Light And Assigning The Dispacted Event Of Change Color To It.
  (`LightComponent.SetLightColor` (`self.PLC_PointLight`) LVAR_LNC_ChangingColor true))

(event `UMEVE_ToggleVisibiltyOFFForDefaultMode`
  (params (LVAR_FL_PlayRate :type "Float (double-precision)"))
  ;[0.02604 0.01891 0] Toggle Visibility Off For Defualt Mode Using Timeline
  ;;[0 0 0] Check Whether The Light Is Off Or Not
  (if (!= (`LightComponentBase.Intensity` (`self.PLC_PointLight`)) 0.0)
    (`TimelineComponent.SetPlayRate` (`self.TMLNC_ToggleVisibiltyOffForDefaultMode`) LVAR_FL_PlayRate)
    (bind (_direction _interpvalue) (`Timeline|TMLNC_ToggleVisibiltyOffForDefaultMode` :!via `PlayFromStart`)
      (:`Update`
        (`LightComponent.SetIntensity` (`self.PLC_PointLight`) (* _interpvalue (`self.TEMP_GlobalIntesity`)))))))

(event `UMEVE_ToggleVisibiltyOnForDefaultMode`
  (params (LVAR_FL_PlayRate :type "Float (double-precision)"))
  ;[0 0 0.0625 1 15] Toggling Visibilty On For Default Mode
  ;;[0 0 0 1 12] Checking Whether Its Is Fully Illuminated Or Not
  (if (!= (`LightComponentBase.Intensity` (`self.PLC_PointLight`)) (`self.TEMP_GlobalIntesity`))
    (`TimelineComponent.SetPlayRate` (`self.TMLNC_ToggleVisibilyOnForDefaultMode`) LVAR_FL_PlayRate)
    (bind (_direction _interpvalue) (`Timeline|TMLNC_ToggleVisibilyOnForDefaultMode` :!via `PlayFromStart`)
      (:`Update`
        (`LightComponent.SetIntensity` (`self.PLC_PointLight`) (* _interpvalue (`self.TEMP_GlobalIntesity`)))))))

(event `self.ReceiveBeginPlay`
  ;[1 1 1] Comment
  (set `self.GVAR_GMO_GameModeSoftRefrence` (`GameplayStatics.GetGameMode`)))

(event `UMEVE_ToggleVIsiblityOnForSnakeMOvement`
  (params (LVAR_FL_PlayRate :type "Float (double-precision)") (LVAR_INT_SnakesIndexNumber :type Integer))
  (bind _temp_globalintesity (`self.TEMP_GlobalIntesity`))
  ;[0.09896 0 0 1 25] Toggle Visiblity On For The Snake Lightiing Mode
  ;;[0.3843 0.1647 0.05882] Checking If The Point Light Is Already Illuminated Or Near To Full Illumination
  (if (`KismetMathLibrary.InRange_FloatFloat` (`LightComponentBase.Intensity` (`self.PLC_PointLight`)) (- _temp_globalintesity 500.0) _temp_globalintesity)
    ;;[0.02222 0.1094 0.02222] Illuminate The Visibilty On Using The TimeLine And Specific Play Rate
    (`TimelineComponent.SetPlayRate` (`self.TMLNC_ToggleVisibilyOnForSnakeMode`) LVAR_FL_PlayRate)
    (bind (_direction _newtrack_0) (`Timeline|TMLNC_ToggleVisibilyOnForSnakeMode` :!via `PlayFromStart`)
      (:`Update`
        (`LightComponent.SetIntensity` (`self.PLC_PointLight`) (* _newtrack_0 (`self.TEMP_GlobalIntesity`))))
      (:`Finished`
        ;;[0.1667 0 0.04579] After Finishing The Visibilty On :-Call The Update Function In game Mode To Notify Its is Done
        (message `/Game/GameContent/BlueprintInterface/UMBINF_SnakeMovementComponent_GameMode/UMBINF_SnakeMovementComponent_GameMode_ACTPointlightBP.INFUN_VisibilityOnDone` (`self.GVAR_GMO_GameModeSoftRefrence`) LVAR_INT_SnakesIndexNumber)))
    (else
      ;;[0.03209 0 0.1302] If The Point Light is Already Illuminated Then Wating For A Delay Of Calculated Time And Then Notifying The Game Mode
      (`KismetSystemLibrary.Delay` (/ 1.0 LVAR_FL_PlayRate))
      (message `/Game/GameContent/BlueprintInterface/UMBINF_SnakeMovementComponent_GameMode/UMBINF_SnakeMovementComponent_GameMode_ACTPointlightBP.INFUN_VisibilityOnDone` (`self.GVAR_GMO_GameModeSoftRefrence`) LVAR_INT_SnakesIndexNumber))))

(event `UMEVE_ToggleVisibiltyOffForSnakeMOde`
  (params (LVAR_FL_PLayRate :type "Float (double-precision)") (LVAR_INT_SnakesIndexNumber :type Integer))
  ;[0 0 0] Toggle Visibilty Off For Snake Ligthing Mode :-Using Timeline
  ;;[0.3843 0.1647 0.05882] Checking If The Point Light Is Already Illuminated Off Near To Be Off
  (if (`KismetMathLibrary.InRange_FloatFloat` (`LightComponentBase.Intensity` (`self.PLC_PointLight`)) 0.0 500.0)
    ;;[0.02222 0.1094 0.02222] Illuminate The Visibilty Off Using The TimeLine And Specific Play Rate
    (`TimelineComponent.SetPlayRate` (`self.TMLNC_ToggleVisibilyOnForSnakeMode`) 0.0)
    (bind (_direction _newtrack_0) (`Timeline|TMLNC_ToggleVisibilityOffForSnakeEffect` :!via `PlayFromStart`)
      (:`Update`
        (`LightComponent.SetIntensity` (`self.PLC_PointLight`) (* _newtrack_0 (`self.TEMP_GlobalIntesity`))))
      (:`Finished`
        ;;[0.1667 0 0.04579] After Finishing The Visibilty Off :-Call The Update Function In game Mode To Notify Its is Done
        (message `/Game/GameContent/BlueprintInterface/UMBINF_SnakeMovementComponent_GameMode/UMBINF_SnakeMovementComponent_GameMode_ACTPointlightBP.INFUN_VIsibiltyOffDone` (`self.GVAR_GMO_GameModeSoftRefrence`) LVAR_INT_SnakesIndexNumber)))
    (else
      ;;[0.03209 0 0.1302] If The Point Light is Already Off Then Wating For A Delay Of Calculated Time And Then Notifying The Game Mode
      (`KismetSystemLibrary.Delay` (/ 1.0 LVAR_FL_PLayRate))
      (message `/Game/GameContent/BlueprintInterface/UMBINF_SnakeMovementComponent_GameMode/UMBINF_SnakeMovementComponent_GameMode_ACTPointlightBP.INFUN_VisibilityOnDone` (`self.GVAR_GMO_GameModeSoftRefrence`) LVAR_INT_SnakesIndexNumber))))

(event `UMEVE_ToggleVisibiltyOnForBreathingEffect`
  (params (LVAR_FL_PlayRate :type "Float (double-precision)"))
  ;[0 0.7365 1] Toggling Visibilty On For Breathing Effect :-Using Timeline
  (`TimelineComponent.SetPlayRate` (`self.TMLNC_ToggleVisibiltyOnForBreathingEffect`) LVAR_FL_PlayRate)
  (bind (_direction _interpvalue) (`Timeline|TMLNC_ToggleVisibiltyOnForBreathingEffect` :!via `PlayFromStart`)
    (:`Update`
      (`LightComponent.SetIntensity` (`self.PLC_PointLight`) (* _interpvalue (`self.TEMP_GlobalIntesity`))))))

(event `UMEVE_ToggleVisibiltyOFFForBreathingEffect`
  (params (LVAR_FL_PLayRate :type "Float (double-precision)"))
  ;[0 1 0.3475] Toggling Visibilty Off For Breathing Effect:-Using Timeline
  (`TimelineComponent.SetPlayRate` (`self.TMLNC_ToggleVisibiltyOffForDefaultMode`) LVAR_FL_PLayRate)
  (bind (_direction _interpvalue) (`Timeline|TMLNC_ToggleVisibiltyOffBreathingEffect` :!via `PlayFromStart`)
    (:`Update`
      (`LightComponent.SetIntensity` (`self.PLC_PointLight`) (* _interpvalue (`self.TEMP_GlobalIntesity`))))))

(fn `UserConstructionScript`)