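; ACT_Key_BP is a key actor, apparently for a keyboard, that spawns ACT_KeyLights_BP actors just beneath itself on BeginPlay.
; It switches on its display name, spawning one light by default and looping to spawn several for the wider R Shift and Space keys.
; The loops use an X offset reset to zero, but the nodes that would increment it and store the spawned references are disconnected.
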(event `self.ReceiveBeginPlay`
  (switch `string` (`KismetSystemLibrary.GetDisplayName` self)
    (:`Default`
      (`|SpawnActorFromClass` "/Game/GameContent/Actors/ACT_KeyLights/ACT_KeyLights_BP.ACT_KeyLights_BP_C" (`KismetMathLibrary.MakeTransform` (`KismetMathLibrary.MakeVector` (.x (.location (`SceneComponent.K2_GetComponentToWorld` (`self.DefaultSceneRoot`)))) (.y (.location (`SceneComponent.K2_GetComponentToWorld` (`self.DefaultSceneRoot`)))) (- (.z (.location (`SceneComponent.K2_GetComponentToWorld` (`self.DefaultSceneRoot`)))) 13.0)) (.rotation (`SceneComponent.K2_GetComponentToWorld` (`self.DefaultSceneRoot`))) (.scale (`SceneComponent.K2_GetComponentToWorld` (`self.DefaultSceneRoot`)))) "Undefined" "OverrideRootScale" null null))
    (:`RShift`
      (set `self.GVAR_INT_NewLocationsOfPointsLight` 0.0)
      (for _ (range 2)
        (`|SpawnActorFromClass` "/Game/GameContent/Actors/ACT_KeyLights/ACT_KeyLights_BP.ACT_KeyLights_BP_C" (`KismetMathLibrary.MakeTransform` (`KismetMathLibrary.MakeVector` (+ (.x (.location (`SceneComponent.K2_GetComponentToWorld` (`self.DefaultSceneRoot`)))) (`self.GVAR_INT_NewLocationsOfPointsLight`)) (.y (.location (`SceneComponent.K2_GetComponentToWorld` (`self.DefaultSceneRoot`)))) (- (.z (.location (`SceneComponent.K2_GetComponentToWorld` (`self.DefaultSceneRoot`)))) 13.0)) (.rotation (`SceneComponent.K2_GetComponentToWorld` (`self.DefaultSceneRoot`))) (.scale (`SceneComponent.K2_GetComponentToWorld` (`self.DefaultSceneRoot`)))) "Undefined" "OverrideRootScale" null null)))
    (:`Space`
      (set `self.GVAR_INT_NewLocationsOfPointsLight` 0.0)
      (for _ (range 6)
        (`|SpawnActorFromClass` "/Game/GameContent/Actors/ACT_KeyLights/ACT_KeyLights_BP.ACT_KeyLights_BP_C" (`KismetMathLibrary.MakeTransform` (`KismetMathLibrary.MakeVector` (+ (.x (.location (`SceneComponent.K2_GetComponentToWorld` (`self.DefaultSceneRoot`)))) (`self.GVAR_INT_NewLocationsOfPointsLight`)) (.y (.location (`SceneComponent.K2_GetComponentToWorld` (`self.DefaultSceneRoot`)))) (- (.z (.location (`SceneComponent.K2_GetComponentToWorld` (`self.DefaultSceneRoot`)))) 13.0)) (.rotation (`SceneComponent.K2_GetComponentToWorld` (`self.DefaultSceneRoot`))) (.scale (`SceneComponent.K2_GetComponentToWorld` (`self.DefaultSceneRoot`)))) "Undefined" "OverrideRootScale" null null)))))

(fn `UserConstructionScript`)