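; Light effect actor that makes its point light "breathe" by endlessly cycling through a spectrum of three colors.
; The construction script applies the first color, and BeginPlay starts the cycle after a short delay.
; A function picks the current and next colors with a wrapping index, assuming exactly three entries.
; A timeline blends them in HSV space, then increments the index and repeats after a pause.
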(event `self.ReceiveBeginPlay`
  (`KismetSystemLibrary.Delay` 0.75)
  (`self.PMF_ChnageTheLightColors`))

(event `EVE_LerpBetweenLightColor`
  (params (IntialColor :type "LinearColor Structure") (FinalColor :type "LinearColor Structure"))
  (bind (_direction _lerpbetweencolorsgraph) (`Timeline|LerpBetweenColorTimeline` :!via `PlayFromStart`)
    (:`Update`
      (`LightComponent.SetLightColor` (`self.PointLight`) (`KismetMathLibrary.LinearColorLerpUsingHSV` IntialColor FinalColor _lerpbetweencolorsgraph) true))
    (:`Finished`
      (`/Engine/EditorBlueprintResources/StandardMacros.IncrementInt` (`self.StartingColourIndex`)
        (:`  `
          (`KismetSystemLibrary.Delay` 0.75)
          (`self.PMF_ChnageTheLightColors`))))))

(fn `PMF_ChnageTheLightColors`
  (if (== (`self.StartingColourIndex`) 3)
    (set `self.StartingColourIndex` 0))
  (`self.EVE_LerpBetweenLightColor` (`|GetArrayItem` (`self.ARR_LC_BreathingColorsSpectrum`) (`self.StartingColourIndex`)) (`|GetArrayItem` (`self.ARR_LC_BreathingColorsSpectrum`) (mod (+ (`self.StartingColourIndex`) 1) 3))))

(fn `UserConstructionScript`
  ;[0 0.488 0] Setting the point light color as the First Light of Breathing Spectrum
  (`LightComponent.SetLightColor` (`self.PointLight`) (`|GetArrayItem` (`self.ARR_LC_BreathingColorsSpectrum`)) true))