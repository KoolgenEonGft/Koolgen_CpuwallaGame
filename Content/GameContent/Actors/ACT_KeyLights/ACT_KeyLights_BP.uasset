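; ACT_KeyLights is a point light actor that runs a looping breathing effect while cycling through an array of colors.
; Two timelines chain to ramp intensity up, then down, scaled by 3000.
; Each completed fade-out calls UMFHandleBreathingEffectWorking, which applies the current color, restarts the fade-in and advances the color index with wraparound.
; BeginPlay is empty, so nothing in this Blueprint starts the loop.
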(event `self.ReceiveBeginPlay`)

(event `UMEVE_ToggleVisibiltyOn`
  (bind (_direction _interpvalue) (`Timeline|TMLNC_ToggleVisibiltyOn` :!via `PlayFromStart`)
    (:`Update`
      (`LightComponent.SetIntensity` (`self.PLNC_PointLightComponent`) (* _interpvalue 3000.0)))
    (:`Finished`
      (`self.UMEVE_ToogleVisibilyOff`))))

(event `UMEVE_ToogleVisibilyOff`
  (bind (_direction _interpvalue) (`Timeline|TMLNC_ToggleVisibiltyOff` :!via `PlayFromStart`)
    (:`Update`
      (`LightComponent.SetIntensity` (`self.PLNC_PointLightComponent`) (* _interpvalue 3000.0)))
    (:`Finished`
      (`self.UMF_HandleBreathingEffectWorking`))))

(fn `UMF_HandleBreathingEffectWorking`
  (bind _returnvalue (+ (`self.GVAR_INT_PresentColorIndex`) 1))
  (`LightComponent.SetLightColor` (`self.PLNC_PointLightComponent`) (`|GetArrayItem` (`self.GARR_LNC_ColorSpectrum`) (`self.GVAR_INT_PresentColorIndex`)) true)
  (`self.UMEVE_ToggleVisibiltyOn`)
  (if (<= _returnvalue (- (`KismetArrayLibrary.Array_Length` (`self.GARR_LNC_ColorSpectrum`)) 1))
    (set `self.GVAR_INT_PresentColorIndex` _returnvalue)
    (else
      (set `self.GVAR_INT_PresentColorIndex` 0))))

(fn `UserConstructionScript`)